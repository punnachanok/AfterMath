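; Zlorp enemy character Blueprint that keeps its health bar widget in sync with its health.
; On BeginPlay it casts the health widget component's widget to WBP_EnemyHealth and binds to its own OnHealthChanged dispatcher, reached through the movement component's pawn owner.
; Each change sets the progress bar percent, assuming a fixed maximum health of 100.
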(event `self.ReceiveBeginPlay`
  (bind _aswbp_enemy_health (cast `/Game/Blueprints/UI/Widgets/Enemies/WBP_EnemyHealth` (`WidgetComponent.GetWidget` (`self.HealthWidget`)))
    (:`then`
      (bind _asbp_zlorp_enemy_character (cast `/Game/Blueprints/Character/Enemies/BP_ZlorpEnemyCharacter` (`PawnMovementComponent.GetPawnOwner` (`self.CharacterMovement`))))
      (add `self.OnHealthChanged` _asbp_zlorp_enemy_character (delegate `OnHealthChanged_Event`)))
    (:`CastFailed`
      (`KismetSystemLibrary.PrintString` "Cast to WBP_EnemyHealth Failed!"))))

(event `OnHealthChanged_Event` :!signature `self.OnHealthChanged`
  (params (NewEnemyHealth :type "Float (single-precision)"))
  (`ProgressBar.SetPercent` (`/Game/Blueprints/UI/Widgets/Enemies/WBP_EnemyHealth.ProgressBar_66` (stale `self.ReceiveBeginPlay` _aswbp_enemy_health)) (/ NewEnemyHealth 100.0)))

(fn `UserConstructionScript`)